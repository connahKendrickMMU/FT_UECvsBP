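; BPTimeLoop is a test actor that times a Blueprint for-loop when another actor overlaps it.
; On BeginPlay, its text render displays the configured loop count.
; On overlap, it prints every index from zero through LoopCount inclusive, then prints the elapsed real time.
; The measurement includes the PrintString cost and subtracts only the PartialSeconds of two GetAccurateRealTime readings, ignoring whole seconds.
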(event `self.ReceiveBeginPlay`
  (`TextRenderComponent.K2_SetText` (`self.TextRender`) (`KismetTextLibrary.Conv_StringToText` (`KismetStringLibrary.Concat_StrStr` "loops " (`KismetStringLibrary.Conv_IntToString` (`self.LoopCount`))))))

(event `self.ReceiveActorBeginOverlap`
  (params (OtherActor :type "Actor Object Reference"))
  (set `self.StartTime` (`.PartialSeconds` (`GameplayStatics.GetAccurateRealTime`)))
  (for _index (range (+ (`self.LoopCount`) 1))
    (`KismetSystemLibrary.PrintString` (`KismetStringLibrary.Concat_StrStr` "loop index" (`KismetStringLibrary.Conv_IntToString` _index))))
  (set `self.EndTime` (`.PartialSeconds` (`GameplayStatics.GetAccurateRealTime`)))
  (`KismetSystemLibrary.PrintString` (`KismetStringLibrary.Concat_StrStr` "loop time" (`KismetStringLibrary.Conv_DoubleToString` (- (`self.EndTime`) (`self.StartTime`))))))

(fn `UserConstructionScript`)